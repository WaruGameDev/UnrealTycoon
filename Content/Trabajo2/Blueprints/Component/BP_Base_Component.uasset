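; Actor component that lets the player pay money toward constructing a building at its owner actor.
; AddMoney checks that the player controller can afford the amount, deducts it and adds it to the resource count.
; Once the count reaches the needed total, BuildBuilding unhides the target building, then hides the owner and disables its collision.
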(fn BuildBuilding
  (bind _returnvalue (Components|GetOwner))
  (Rendering|SetActorHiddenInGame (Variables|Default|GetBuildingToActivate) false)
  (Collision|SetActorEnableCollision _returnvalue false)
  (Rendering|SetActorHiddenInGame _returnvalue true))

(fn AddMoney
  (params (Count :type Integer) (PlayerController :type BP%20Top%20Down%20Controller%20Object%20Reference))
  (if (>= (Variables|/Game/TopDown/Blueprints/BP_TopDownController.BP_TopDownController_C|GetMoney PlayerController) Count)
    (Default|ChangeMoney PlayerController (* Count -1))
    (bind _output_get (Variables|Default|SetResourceCount (+ (Variables|Default|GetResourceCount) Count)))
    (if (>= _output_get (Variables|Default|GetResourseNeededCount))
      (CallFunction|BuildBuilding))))