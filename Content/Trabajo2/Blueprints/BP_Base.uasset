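; BP_Base is a zone actor that repeatedly triggers a money transaction while the player stays inside it.
; Entering the zone caches the BP_TopDownController and, if its Money is non-negative, starts the AddMoney timeline.
; Each time the timeline finishes, it calls AddMoney on BPBaseComponent with that controller, then restarts without rechecking Money.
; Leaving the zone clears the presence flag and stops the timeline.
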(event EventOnCollideBegin
  (Variables|Default|SetIsPlayerInZone true)
  (Variables|Default|GetAs%20BP%20Top%20Down%20Controller
    (:then
      _)
    (:else
      (Variables|Default|SetAs%20BP%20Top%20Down%20Controller (.AsBP%20Top%20Down%20Controller (Utilities|Casting|CastToBP_TopDownController (Game|GetPlayerController 0))))))
  (if (>= (Variables|/Game/TopDown/Blueprints/BP_TopDownController.BP_TopDownController_C|GetMoney (Variables|Default|GetAs%20BP%20Top%20Down%20Controller)) 0)
    (Timeline|AddMoney PlayFromStart
      (:Finished
        (Default|AddMoney (Variables|Default|GetBP_Base_Component) 1 (Variables|Default|GetAs%20BP%20Top%20Down%20Controller))
        (if (Variables|Default|GetIsPlayerInZone)
          (Timeline|AddMoney PlayFromStart))))))

(event EventOnCollideEnd
  (Variables|Default|SetIsPlayerInZone false)
  (Timeline|AddMoney Stop
    (:Finished
      (Default|AddMoney (Variables|Default|GetBP_Base_Component) 1 (Variables|Default|GetAs%20BP%20Top%20Down%20Controller))
      (if (Variables|Default|GetIsPlayerInZone)
        (Timeline|AddMoney PlayFromStart)))))

(fn ConstructionScript)