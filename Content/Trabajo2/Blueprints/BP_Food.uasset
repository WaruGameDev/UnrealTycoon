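; BP_Food is a food item actor that displays a model, name, price and sell price taken from a data table.
; The Construction Script reads the row selected by the FoodData row handle, sets the static mesh and three text renders, and stores Price in a variable.
; On BeginPlay, it loops over every row in that table and prints each food name, regardless of the selected row.
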(event EventBeginPlay
  (bind _food_data (Variables|Default|GetFood%20Data))
  (bind _outrownames (DataTable|GetDataTableRowNames (.datatable _food_data)))
  (for _array_element _outrownames
    (bind _returnvalue (Utilities|GetDataTableRow (.datatable _food_data) _array_element)
      (:then
        (Development|PrintString (.FoodName (Utilities|Struct|BreakS_Food _returnvalue)))))))

(event Collision|EventActorBeginOverlap
  (params (OtherActor :type Actor%20Object%20Reference)))

(event EventTick
  (params (DeltaSeconds :type Float%20%28single-precision%29)))

(fn ConstructionScript
  (bind _food_data (Variables|Default|GetFood_Data))
  (bind _returnvalue (Utilities|GetDataTableRow (.datatable _food_data) (.rowname _food_data))
    (:then
      (Components|StaticMesh|SetStaticMesh (Variables|Default|GetStaticMesh) (.FoodModel (Utilities|Struct|BreakS_Food _returnvalue)))
      (Rendering|Components|TextRender|SetText (Variables|Default|GetTextRender) (Utilities|Text|ToText(String) (.FoodName (Utilities|Struct|BreakS_Food _returnvalue))))
      (Rendering|Components|TextRender|SetText (Variables|Default|GetTextRender1) (Utilities|Text|ToText(String) (Utilities|String|Append "$" (Utilities|String|ToString(Integer) (.Price (Utilities|Struct|BreakS_Food _returnvalue))))))
      (Rendering|Components|TextRender|SetText (Variables|Default|GetTextRender2) (Utilities|Text|ToText(String) (Utilities|String|Append "$" (Utilities|String|ToString(Integer) (.SellPrice (Utilities|Struct|BreakS_Food _returnvalue))))))
      (Variables|Default|SetPrice (.Price (Utilities|Struct|BreakS_Food _returnvalue))))))